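; Lobby game mode that keeps the list of connected player controllers and keeps every client's lobby roster up to date.
; PostLogin (after a short delay, on authority) and OnLogout edit AllPcs, then call UpdateServer.
; UpdateServer rebuilds name and index arrays and pushes them, then the player count, to each BP_S1LobbyPlayerController.
; KickPlayer uses that same index to call Kick on the chosen controller.
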(event Custom|UpdateServer
  (bind _all_pcs (Variables|Default|GetAll%20Pcs))
  (for _array_element (Variables|Default|GetAll%20Pcs)
    (bind _asbp_s1lobby_pc (Utilities|Casting|CastToBP_S1LobbyPlayerController _array_element))
    (Utilities|Array|Clear (Variables|Default|GetTextArr))
    (Utilities|Array|Clear (Variables|Default|GetIdxArr))
    (for (_array_element_2 _array_index) (Variables|Default|GetAll%20Pcs)
      (Utilities|Array|Add (Variables|Default|GetTextArr) (Utilities|Text|ToText(String) (Class|AdvancedSessionsLibrary|GetPlayerName _array_element_2)))
      (Utilities|Array|Add (Variables|Default|GetIdxArr) _array_index))
    (Default|AddPlayer _asbp_s1lobby_pc (Variables|Default|GetTextArr) (Variables|Default|GetIdxArr)))
  (for _array_element_3 _all_pcs
    (bind _asbp_s1lobby_pc_2 (Utilities|Casting|CastToBP_S1LobbyPlayerController _array_element_3))
    (Default|UpdateNumOfPlayers _asbp_s1lobby_pc_2 (Utilities|Array|Length _all_pcs))))

(event Custom|KickPlayer
  (params (Idx :type Integer))
  (bind _asbp_s1lobby_pc (Utilities|Casting|CastToBP_S1LobbyPlayerController (Utilities|Array|Get(acopy) (Variables|Default|GetAll%20Pcs) Idx)))
  (Default|Kick _asbp_s1lobby_pc))

(event EventBeginPlay
  (bind _asbp_s1gi (Utilities|Casting|CastToBP_S1GI (Game|GetGameInstance)))
  (Variables|Default|SetAs%20BP%20S1GI _asbp_s1gi))

(event EventPostLogin
  (params (NewPlayer :type Player%20Controller%20Object%20Reference))
  (Utilities|FlowControl|Delay 0.1)
  (Networking|SwitchHasAuthority
    (:Authority
      (Utilities|Array|Add (Variables|Default|GetAll%20Pcs) NewPlayer)
      (CallFunction|UpdateServer))))

(event EventOnLogout
  (params (ExitingController :type Controller%20Object%20Reference))
  (bind _all_pcs (Variables|Default|GetAll%20Pcs))
  (bind (_array_element _array_index) (Utilities|Array|ForEachLoopwithBreak _all_pcs :!label _label)
    (:LoopBody
      (if (== _array_element ExitingController)
        (goto _label Break)))
    (:Completed
      (Utilities|Array|RemoveIndex _all_pcs _array_index)
      (CallFunction|UpdateServer))))

(fn ConstructionScript)