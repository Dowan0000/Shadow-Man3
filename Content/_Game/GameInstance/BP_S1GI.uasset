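; Game instance that runs Steam multiplayer sessions through Advanced Sessions nodes and owns the main menu, create-session, session-list and loading-screen widgets.
; Creating a session opens LobbyLevel as a listen server behind a loading screen.
; Searches cache results for the session-list widget, created on first use and reloaded on refresh.
; Joins, including accepted invites, show the loading screen and refresh the list on failure.
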(event Custom|Refresh%20Session%20List
  (bind _session_list (Variables|Default|GetSession%20List))
  (Utilities|Array|Clear (Variables|Default|GetResults))
  (bind _results (|FindSessionsAdvanced (Game|GetPlayerController 0) 1000 false "AllServers" 0 false false false true)
    (:OnSuccess
      (bind _output_get (Variables|Default|SetResults _results))
      (Utilities|IsValid _session_list
        (:Is%20Valid
          (Default|LoadSessionList _session_list _output_get))))))

(event EventShowSessionList
  (params (Sessions :type Array%20of%20Blueprint%20Session%20Result%20Structures))
  (bind _returnvalue (Game|GetPlayerController 0))
  ;[1 1 1] Show Session List
  (Variables|Default|GetSession%20List
    (:then
      _)
    (:else
      (bind _returnvalue_2 (UserInterface|CreateWidget "/Game/_Game/UI/Session/WBP_SessionList.WBP_SessionList_C" _returnvalue Sessions))
      (Variables|Default|SetSession%20List _returnvalue_2)))
  (UserInterface|Viewport|AddtoViewport (Variables|Default|GetSession%20List) 0)
  (Variables|/Script/Engine.PlayerController|SetbShowMouseCursor _returnvalue true))

(event EventFindSteamSession
  ;[1 1 1] Find Session
  (Utilities|Array|Clear (Variables|Default|GetResults))
  (bind _results (|FindSessionsAdvanced (Game|GetPlayerController 0) 1000 false "AllServers" 0 false false false true)
    (:OnSuccess
      (bind _output_get (Variables|Default|SetResults _results))
      (CallFunction|ShowSessionList _output_get))))

(event EventJoinSteamSession
  (params (SessionToJoin :type Blueprint%20Session%20Result%20Structure))
  ;[1 1 1] Join Session
  (CallFunction|ShowLoadingScreen)
  (|JoinSession (Game|GetPlayerController 0) SessionToJoin
    (:OnSuccess
      (Development|PrintString "////////// Join Session //////////" true true "(R=0.012269,G=1.000000,B=0.000000,A=1.000000)"))
    (:OnFailure
      (Development|PrintString "////////// Join Fail //////////" true true "(R=1.000000,G=0.030793,B=0.000000,A=1.000000)")
      (CallFunction|RefreshSessionList))))

(event EventOnSessionInviteAccepted
  (params (LocalPlayerNum :type Integer) (PersonInvited :type BP%20Unique%20Net%20Id%20Structure) (SessionToJoin :type Blueprint%20Session%20Result%20Structure%20%28by%20ref%29))
  ;[1 1 1] 코멘트
  (CallFunction|JoinSteamSession SessionToJoin))

(event EventShowCreateSession
  (bind _returnvalue (Game|GetPlayerController 0))
  ;[1 1 1] Show Create Widget
  (Variables|Default|GetWBP_CreateSession
    (:then
      _)
    (:else
      (bind _returnvalue_2 (UserInterface|CreateWidget "/Game/_Game/UI/Session/WBP_CreateSession.WBP_CreateSession_C" _returnvalue))
      (Variables|Default|SetWBP_CreateSession _returnvalue_2)))
  (UserInterface|Viewport|AddtoViewport (Variables|Default|GetWBP_CreateSession) 0)
  (Variables|/Script/Engine.PlayerController|SetbShowMouseCursor _returnvalue true))

(event EventShowMainMenu
  ;[1 1 1] Show MainMenu
  (Variables|Default|GetWBP_MainMenu
    (:then
      _)
    (:else
      (bind _returnvalue (UserInterface|CreateWidget "/Game/_Game/UI/WBP_MainMenu.WBP_MainMenu_C" (Game|GetPlayerController 0)))
      (Variables|Default|SetWBP_MainMenu _returnvalue)))
  (UserInterface|Viewport|AddtoViewport (Variables|Default|GetWBP_MainMenu) 0))

(event EventShowLoadingScreen
  ;[1 1 1] Show LoadingScreen
  (Variables|Default|GetWBP_LoadingScreen
    (:then
      _)
    (:else
      (bind _returnvalue (UserInterface|CreateWidget "/Game/_Game/UI/WBP_LoadingScreen.WBP_LoadingScreen_C" (Game|GetPlayerController 0)))
      (Variables|Default|SetWBP_LoadingScreen _returnvalue)))
  (UserInterface|Viewport|AddtoViewport (Variables|Default|GetWBP_LoadingScreen) 0))

(event EventCreateSteamSession
  (params (Public%20Connections :type Integer) (Public%20Session :type Boolean))
  ;[1 1 1] Create Session
  (|AdvancedSession 0 (Game|GetPlayerController 0) Public%20Connections 0 false true false true true true false false false Public%20Session false true
    (:OnSuccess
      (CallFunction|ShowLoadingScreen)
      (Development|PrintString "Create Session")
      (Game|OpenLevel(byName) "LobbyLevel" true "listen"))))

(fn Reference
  (return 0))