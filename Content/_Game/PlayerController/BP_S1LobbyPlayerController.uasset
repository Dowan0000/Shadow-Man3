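; Lobby player controller that owns each player's lobby HUD and handles being kicked from the session.
; BeginPlay caches the game instance, creates the lobby HUD sized for four players and shows the mouse cursor.
; Events relay player count, list clearing and player additions to the HUD, with additions held behind a short Delay marked for later rework.
; Kick opens the main menu level and destroys the session.
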(event Custom|AddPlayer
  (params (PlayerName :type Array%20of%20Texts) (PlayerIdx :type Array%20of%20Integers))
  ;[1 1 1] 나중에 수정
  (Utilities|FlowControl|Delay 0.1)
  (Default|AddPlayertoList (Variables|Default|GetWBP_LobbyHUD) PlayerName PlayerIdx))

(event Custom|ClearPlayerList
  (Default|ClearPlayerList (Variables|Default|GetWBP_LobbyHUD)))

(event Custom|Kick
  (Game|OpenLevel(byName) "MainMenu")
  (|DestroySession self))

(event Custom|UpdateNumOfPlayers
  (params (CurrentPlayers :type Integer))
  (Variables|/Game/_Game/UI/Game/WBP_LobbyHUD.WBP_LobbyHUD_C|SetCurrentPlayers (Variables|Default|GetWBP_LobbyHUD) CurrentPlayers))

(event EventBeginPlay
  (bind _asbp_s1gi (Utilities|Casting|CastToBP_S1GI (Game|GetGameInstance)))
  (Variables|Default|SetAs%20BP%20S1GI _asbp_s1gi)
  (bind _returnvalue (UserInterface|CreateWidget "/Game/_Game/UI/Game/WBP_LobbyHUD.WBP_LobbyHUD_C"))
  (bind _output_get (Variables|Default|SetWBP_LobbyHUD _returnvalue))
  (UserInterface|Viewport|AddtoViewport _output_get 0)
  (Variables|Default|SetbShowMouseCursor true))

(fn ConstructionScript)